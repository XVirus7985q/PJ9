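; Game mode for a chat-based number-guessing game between Host and Guest, holding a random target number created at BeginPlay.
; Client messages have a three-character guess extracted, validated and judged inside a loop over player controllers, which broadcasts the result or "OUT!" to each BP_Controller.
; A correct guess announces a win and calls ResetGame for a new target; a wrong one announces a draw when both try counts are equal.
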(event `self.ReceiveBeginPlay`
  (bind _returnvalue (`MyTestCPPLib.GenerateRandomNumber`))
  (bind _output_get (set `self.TargetNumber` _returnvalue))
  (`KismetSystemLibrary.PrintString` _output_get))

(event `ResetGame`
  (bind _returnvalue (`MyTestCPPLib.GenerateRandomNumber`))
  (set `self.TargetNumber` _returnvalue)
  (bind _outactors (`GameplayStatics.GetAllActorsOfClass` "/Script/Engine.PlayerController"))
  (for _array_element _outactors
    (bind _asbp_controller (cast `/Game/Blueprints/BP_Controller` _array_element))
    (set `/Game/Blueprints/BP_Controller.TryCount_Host` (`/Game/Blueprints/BP_Controller.TryCount_Host` _asbp_controller) _asbp_controller)
    (set `/Game/Blueprints/BP_Controller.TryCount_Guest` (`/Game/Blueprints/BP_Controller.TryCount_Guest` _asbp_controller) _asbp_controller)
    (`/Game/Blueprints/BP_Controller.GotBroadcast` _asbp_controller "\"🔁 새 게임이 시작됩니다!\"")))

(event `GotMessageFromClient`
  (params (Msg :type String) (UserId :type String))
  (bind _targetnumber (`self.TargetNumber`))
  (bind _outactors (`GameplayStatics.GetAllActorsOfClass` "/Script/Engine.PlayerController"))
  (for _array_element _outactors
    (bind _asbp_controller (cast `/Game/Blueprints/BP_Controller` _array_element))
    (bind _output_get (set `self.ExtractedNumber` (`KismetStringLibrary.GetSubstring` (`KismetStringLibrary.Replace` Msg "Host") 2 3)))
    (bind _returnvalue (`MyTestCPPLib.IsValidInput` _output_get))
    (if _returnvalue
      (bind _returnvalue_2 (`MyTestCPPLib.JudgeAnswer` _output_get _targetnumber))
      (`/Game/Blueprints/BP_Controller.GotBroadcast` _asbp_controller _returnvalue_2)
      (bind _returnvalue_3 (`MyTestCPPLib.IsCorrect` _output_get _targetnumber))
      (if _returnvalue_3
        (`/Game/Blueprints/BP_Controller.GotBroadcast` _asbp_controller "\"🎉 Correct! You win! 🎉\"")
        (`self.ResetGame`)
        (else
          (bind _output_get_2 (set `/Game/Blueprints/BP_Controller.TryCount_Host` (`/Game/Blueprints/BP_Controller.TryCount_Host` _asbp_controller) _asbp_controller))
          (`KismetSystemLibrary.PrintString` (`KismetStringLibrary.Conv_IntToString` _output_get_2))
          (bind _output_get_3 (set `/Game/Blueprints/BP_Controller.TryCount_Guest` (`/Game/Blueprints/BP_Controller.TryCount_Guest` _asbp_controller) _asbp_controller))
          (`KismetSystemLibrary.PrintString` (`KismetStringLibrary.Conv_IntToString` _output_get_3))
          (if (== _output_get_2 _output_get_3)
            (`/Game/Blueprints/BP_Controller.GotBroadcast` _asbp_controller "\"무승부!\""))))
      (else
        (`/Game/Blueprints/BP_Controller.GotBroadcast` _asbp_controller "\"OUT!\"")))))

(fn `UserConstructionScript`)